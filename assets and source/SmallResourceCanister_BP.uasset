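; Small Resource Canister, an Astroneer backpack item that stores a few units of one resource type as a count plus type.
; Use toggles load/unload; a self-recalling 0.2s IOLooper moves items between that count, the IO slot and connected storage, pulling only whitelisted types.
; UpdateVisuals refreshes fill bars and tooltip, while placement in a shredder slot respawns and ejects the contents.
; The author marks this storage method as outdated, favouring the Large Liquid canister's setup.
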(event `self.StartInWorld`)

(event `self.ReceiveBeginPlay`
  (`ClickableComponent.SetActiveUseContext` (`self.ClickableComponent`) (select `bool` (`self.Importing?`) :`false` "UC_Unload" :`true` "UC_Load" :!type "EUseContext Enum"))
  (`self.IO Looper`)
  (`self.UpdateVisuals`))

(event `InputAction|Use`
  (params (Key :type "Key Structure"))
  (:`Pressed`
    (if (not (`self.Processing`))
      (bind _output_get (set `self.Importing?` (not (`self.Importing?`))))
      (`ClickableComponent.SetActiveUseContext` (`self.ClickableComponent`) (select `bool` _output_get :`false` "UC_Unload" :`true` "UC_Load" :!type "EUseContext Enum")))))

(event `self.PlacedInSlot`
  (params (Slot :type "SlotReference Structure") (FromTool :type Boolean) (SlottedDuringInitialization :type Boolean))
  (if (== Slot_SlotName "ShreddingSlot")
    (for _ (range 1 (+ (`self.Amount`) 1))
      (`SlotsComponent.SpawnItemTypeInSlot` (`self.IOSlotRef`) (`self.ItemType`) true)
      (`SlotStatics.EjectAllItemsInSubslotAndChildSubslots` (`self.IOSlotRef`)))))

(event `IO Looper`
  (if (`self.Importing?`)
    (if (`self.HasItemInIOSlot`)
      (if (or (and (== (`self.ItemInIOSlot`) (`self.ItemType`)) (< (`self.Amount`) (defaults `/Game/Mods/Milkev/ExpandedCanisters/CanisterCapacities` "/Game/Mods/Milkev/ExpandedCanisters/CanisterCapacities.CanisterCapacities_C"))) (== (`self.Amount`) 0))
        (`/Engine/EditorBlueprintResources/StandardMacros.IncrementInt` (`self.Amount`)
          (:`  `
            (set `self.ItemType` (`self.ItemInIOSlot`))
            (`self.TakeItem`
              (:`Finished`
                _)))))
      (else
        (`self.AttemptObtainItemFromConnectedStorageNetwork`)))
    (elif (`self.HasItemInIOSlot`)
      (if (`.ItemIsFull` (`self.HasItemInIOSlot`))
        (`SlotStatics.AttemptToPlaceItemInConnectedStorageSlotNetwork` (`SlotsComponent.GetSlotItem` (`self.IOSlotRef`)) self))
      (elif (> (`self.Amount`) 0)
        (`/Engine/EditorBlueprintResources/StandardMacros.DecrementInt` (`self.Amount`)
          (:`  `
            (`self.AddItem`
              (:`true`
                (if (== (`self.Amount`) 0)
                  (set `self.ItemType` null))))))
        (else
          (set `self.ItemType` null)))))
  (`self.UpdateVisuals`)
  (`KismetSystemLibrary.Delay` 0.2)
  (`self.IO Looper`))

(fn `GetBodySlotLegacy`
  (returns (ReturnValue :type "ChildSlotComponent Object Reference"))
  (return (`self.Body Slot`)))

(fn `UpdateVisuals`
  (bind _amount (`self.Amount`))
  (bind _staticmeshcomponent (`self.StaticMeshComponent`))
  (bind _staticmeshcomponent_2 (`self.StaticMeshComponent`))
  (bind _staticmeshcomponent_3 (`self.StaticMeshComponent`))
  (bind _staticmeshcomponent_4 (`self.StaticMeshComponent`))
  (bind _staticmeshcomponent_5 (`self.StaticMeshComponent`))
  (bind _returnvalue (`KismetSystemLibrary.GetClassDisplayName` (`self.ItemType`)))
  (if (<= _amount 0)
    (`PrimitiveComponent.SetMaterialByName` _staticmeshcomponent "Bar1" "/Game/Mods/Milkev/ExpandedCanisters/Assets/LightGrey.LightGrey")
    (`PrimitiveComponent.SetMaterialByName` _staticmeshcomponent "Bar2" "/Game/Mods/Milkev/ExpandedCanisters/Assets/LightGrey.LightGrey")
    (`PrimitiveComponent.SetMaterialByName` _staticmeshcomponent "Bar3" "/Game/Mods/Milkev/ExpandedCanisters/Assets/LightGrey.LightGrey")
    (`PrimitiveComponent.SetMaterialByName` _staticmeshcomponent "Bar4" "/Game/Mods/Milkev/ExpandedCanisters/Assets/LightGrey.LightGrey")
    (elif (== _amount 1)
      (`PrimitiveComponent.SetMaterialByName` _staticmeshcomponent_5 "Bar1" "/Game/Mods/Milkev/ExpandedCanisters/Assets/BlueHighlight.BlueHighlight")
      (`PrimitiveComponent.SetMaterialByName` _staticmeshcomponent_5 "Bar2" "/Game/Mods/Milkev/ExpandedCanisters/Assets/LightGrey.LightGrey")
      (`PrimitiveComponent.SetMaterialByName` _staticmeshcomponent_5 "Bar3" "/Game/Mods/Milkev/ExpandedCanisters/Assets/LightGrey.LightGrey")
      (`PrimitiveComponent.SetMaterialByName` _staticmeshcomponent_5 "Bar4" "/Game/Mods/Milkev/ExpandedCanisters/Assets/LightGrey.LightGrey")
      (elif (== _amount 2)
        (`PrimitiveComponent.SetMaterialByName` _staticmeshcomponent_4 "Bar1" "/Game/Mods/Milkev/ExpandedCanisters/Assets/BlueHighlight.BlueHighlight")
        (`PrimitiveComponent.SetMaterialByName` _staticmeshcomponent_4 "Bar2" "/Game/Mods/Milkev/ExpandedCanisters/Assets/BlueHighlight.BlueHighlight")
        (`PrimitiveComponent.SetMaterialByName` _staticmeshcomponent_4 "Bar3" "/Game/Mods/Milkev/ExpandedCanisters/Assets/LightGrey.LightGrey")
        (`PrimitiveComponent.SetMaterialByName` _staticmeshcomponent_4 "Bar4" "/Game/Mods/Milkev/ExpandedCanisters/Assets/LightGrey.LightGrey")
        (elif (== _amount 3)
          (`PrimitiveComponent.SetMaterialByName` _staticmeshcomponent_3 "Bar1" "/Game/Mods/Milkev/ExpandedCanisters/Assets/BlueHighlight.BlueHighlight")
          (`PrimitiveComponent.SetMaterialByName` _staticmeshcomponent_3 "Bar2" "/Game/Mods/Milkev/ExpandedCanisters/Assets/BlueHighlight.BlueHighlight")
          (`PrimitiveComponent.SetMaterialByName` _staticmeshcomponent_3 "Bar3" "/Game/Mods/Milkev/ExpandedCanisters/Assets/BlueHighlight.BlueHighlight")
          (`PrimitiveComponent.SetMaterialByName` _staticmeshcomponent_3 "Bar4" "/Game/Mods/Milkev/ExpandedCanisters/Assets/LightGrey.LightGrey")
          (else
            (`PrimitiveComponent.SetMaterialByName` _staticmeshcomponent_2 "Bar1" "/Game/Mods/Milkev/ExpandedCanisters/Assets/BlueHighlight.BlueHighlight")
            (`PrimitiveComponent.SetMaterialByName` _staticmeshcomponent_2 "Bar2" "/Game/Mods/Milkev/ExpandedCanisters/Assets/BlueHighlight.BlueHighlight")
            (`PrimitiveComponent.SetMaterialByName` _staticmeshcomponent_2 "Bar3" "/Game/Mods/Milkev/ExpandedCanisters/Assets/BlueHighlight.BlueHighlight")
            (`PrimitiveComponent.SetMaterialByName` _staticmeshcomponent_2 "Bar4" "/Game/Mods/Milkev/ExpandedCanisters/Assets/BlueHighlight.BlueHighlight"))))))
  (set `TooltipComponent.DefaultDisplayData` (make `TooltipWidgetDisplayData` (`.InteractionPrompts` (break `TooltipWidgetDisplayData` (`TooltipComponent.DefaultDisplayData` (`self.TooltipComponent`)))) (struct) null null (`KismetTextLibrary.Conv_StringToText` (`KismetStringLibrary.Concat_StrStr` "A small canister capable of holding 4 resource. Fits in your backpack! \n \nHolding: " (select `bool` (== (`self.ItemType`) null) :`false` (`KismetStringLibrary.GetSubstring` _returnvalue 0 (- (`KismetStringLibrary.Len` _returnvalue) 2)) :`true` "Nothing") " x " (`KismetStringLibrary.Conv_IntToString` (`self.Amount`)) " / " (`KismetStringLibrary.Conv_IntToString` (defaults `/Game/Mods/Milkev/ExpandedCanisters/CanisterCapacities` "/Game/Mods/Milkev/ExpandedCanisters/CanisterCapacities.CanisterCapacities_C")))) "Small Resource Canister" "Tool") (`self.TooltipComponent`))
  (`ClickableComponent.SetActiveUseContext` (`self.ClickableComponent`) (select `bool` (not (`self.Importing?`)) :`false` "UC_Unload" :`true` "UC_Load" :!type "EUseContext Enum"))
  (`ClickableComponent.SetActiveUseContext` (`self.ClickableComponent`) (select `bool` (`self.Importing?`) :`false` "UC_Unload" :`true` "UC_Load" :!type "EUseContext Enum")))

(fn `UserConstructionScript`
  (bind _staticmeshcomponent (`self.StaticMeshComponent`))
  (set `self.IOSlotRef` (`ChildSlotComponent.MakeReference` (`self.IO Slot`)))
  ;[1 1 1] Section Bars
  (`PrimitiveComponent.SetMaterialByName` _staticmeshcomponent "Bar1" "/Game/Mods/Milkev/ExpandedCanisters/Assets/BlueHighlight.BlueHighlight")
  (`PrimitiveComponent.SetMaterialByName` _staticmeshcomponent "Bar2" "/Game/Mods/Milkev/ExpandedCanisters/Assets/BlueHighlight.BlueHighlight")
  (`PrimitiveComponent.SetMaterialByName` _staticmeshcomponent "Bar3" "/Game/Mods/Milkev/ExpandedCanisters/Assets/BlueHighlight.BlueHighlight")
  (`PrimitiveComponent.SetMaterialByName` _staticmeshcomponent "Bar4" "/Game/Mods/Milkev/ExpandedCanisters/Assets/BlueHighlight.BlueHighlight"))